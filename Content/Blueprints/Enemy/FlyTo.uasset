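; FlyTo is a behavior tree task that flies an enemy pawn to a wander position read from the blackboard.
; On execute, the AI controller moves straight toward that point without pathfinding.
; Each tick accumulates elapsed time and finishes successfully once the pawn is close to the target or a short timeout passes, so the task succeeds even if the point is never reached.
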(event EventReceiveExecuteAI
  (params (OwnerController :type AI%20Controller%20Object%20Reference) (ControlledPawn :type Pawn%20Object%20Reference))
  (AI|Navigation|MovetoLocation OwnerController (Class|BTFunctionLibrary|GetBlackboardValueasVector (Variables|Default|GetWanderPositionKey)) 1e+01 true false false))

(event EventReceiveTickAI
  (params (OwnerController :type AI%20Controller%20Object%20Reference) (ControlledPawn :type Pawn%20Object%20Reference) (DeltaSeconds :type Float%20%28single-precision%29))
  (bind _output_get (Variables|Default|SetAccumulatedTime (+ DeltaSeconds (Variables|Default|GetAccumulatedTime))))
  (if (or (< (Math|Vector|VectorLength (- (Transformation|GetActorLocation (stale EventReceiveExecuteAI ControlledPawn)) (Class|BTFunctionLibrary|GetBlackboardValueasVector (Variables|Default|GetWanderPositionKey)))) 1e+02) (> _output_get 3.0))
    (AI|BehaviorTree|FinishExecute true)))