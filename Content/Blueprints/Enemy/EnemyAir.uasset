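; EnemyAir is an enemy Blueprint that keeps its body turned relative to the player and fires on a repeating timer.
; BeginPlay starts the looping Fire timer at FireDelay; Fire currently only prints a debug string.
; Every tick it sets EnemyThreeBody's rotation from a look-at toward the player pawn, combined with a 90-degree offset.
; Die extends the parent's death logic by disabling the body's collision.
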(event EventBeginPlay
  (|CallParentFunction)
  (Utilities|Time|SetTimerbyFunctionName 0 "Fire" (Variables|Default|GetFireDelay) true))

(event EventTick
  (params (DeltaSeconds :type Float%20%28single-precision%29))
  (bind _returnvalue (Game|Player|GetPlayerPawn 0))
  (bind _returnvalue_2 (Transformation|GetActorLocation))
  (bind _rootcomponent (Variables|/Script/Engine.Actor|GetRootComponent _returnvalue))
  (bind _returnvalue_3 (Transformation|GetWorldLocation _rootcomponent))
  (bind _returnvalue_4 (Math|Rotator|FindLookatRotation _returnvalue_2 _returnvalue_3))
  (|CallParentFunction DeltaSeconds)
  (Transformation|SetWorldRotation (Variables|Default|Getenemy_three_Body) (Math|Rotator|CombineRotators _returnvalue_4 (Math|Vector|RotatorfromAxisandAngle (Math|Vector|GetUpVector _returnvalue_4) -9e+01)) false false))

(event EventDie
  (|CallParentFunction)
  (Collision|SetCollisionEnabled (Variables|Default|Getenemy_three_Body) "NoCollision"))

(fn ConstructionScript
  (|CallParentFunction))

(fn Fire
  (Development|PrintString "pew!"))