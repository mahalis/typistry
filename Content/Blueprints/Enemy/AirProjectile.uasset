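; AirProjectile is an enemy projectile that damages a WordCharacter on overlap, passing its location as the damage source, then destroys itself.
; It passes through EnemyBase actors and dies on overlapping any other actor.
; Tick also destroys it once it strays too far from the world origin or drops below a fixed height.
; The graphs contain no movement logic.
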(event EventBeginPlay)

(event Collision|EventActorBeginOverlap
  (params (OtherActor :type Actor%20Object%20Reference))
  (bind _asword_character (Utilities|Casting|CastToWordCharacter OtherActor)
    (:then
      (Default|Hurt _asword_character 20 (Transformation|GetActorLocation))
      (CallFunction|Die))
    (:CastFailed
      (Utilities|Casting|CastToEnemyBase OtherActor
        (:CastFailed
          (CallFunction|Die))))))

(event EventTick
  (params (DeltaSeconds :type Float%20%28single-precision%29))
  (bind _returnvalue (Transformation|GetActorLocation))
  (if (or (>= (Math|Vector|VectorLength _returnvalue) 4.4e+03) (< (.Z (Math|Vector|BreakVector _returnvalue)) -565.0))
    (CallFunction|Die)))

(fn ConstructionScript)

(fn Die
  (Actor|DestroyActor))