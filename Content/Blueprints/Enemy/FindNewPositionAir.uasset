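; Behavior tree task that picks a new wander position for an airborne enemy around the player.
; On execute, it flattens and normalizes random unit vector components into a horizontal direction, scales it by a random distance and offsets it from the player pawn's location with a random upward height.
; It writes the point to the wander position blackboard key and finishes successfully at once, with no navigation or collision check.
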(event EventReceiveExecuteAI
  (params (OwnerController :type AI%20Controller%20Object%20Reference) (ControlledPawn :type Pawn%20Object%20Reference))
  (bind _returnvalue (Math|Random|RandomUnitVector))
  (AI|BehaviorTree|SetBlackboardValueasVector (Variables|Default|GetWanderPositionKey) (+ (* (Math|Vector|Normalize (Math|Vector|MakeVector (.x _returnvalue) (.y _returnvalue) 0.0)) (Math|Random|RandomFloatinRange 6e+02 1.2e+03)) (Transformation|GetActorLocation (Game|Player|GetPlayerPawn 0)) (Math|Vector|MakeVector 0.0 0.0 (Math|Random|RandomFloatinRange 1e+01 2e+02))))
  (AI|BehaviorTree|FinishExecute true))