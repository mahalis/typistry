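; Base enemy Blueprint for a word-based game that gives each enemy its own set of random words.
; On BeginPlay it copies base health into current health, then calls RetrieveWords.
; RetrieveWords pulls three words from the WordGameMode word list, passing a value derived from base health that steps down per word, with a floor of three.
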(event EventBeginPlay
  (Variables|Default|SetCurrentHealth (Variables|Default|GetBaseHealth))
  (CallFunction|RetrieveWords))

(event Collision|EventActorBeginOverlap
  (params (OtherActor :type Actor%20Object%20Reference)))

(event EventTick
  (params (DeltaSeconds :type Float%20%28single-precision%29)))

(fn ConstructionScript)

(fn RetrieveWords
  (bind _asword_game_mode (Utilities|Casting|CastToWordGameMode (Game|GetGameMode)))
  (for _index (range 0 2)
    (bind _word (Default|RandomWordfromWordList _asword_game_mode (Math|Integer|Max(Integer) (- (Variables|Default|GetBaseHealth) _index) 3)))
    (Utilities|Array|Add (Variables|Default|GetWords) _word)))