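; Behavior tree service that checks whether the AI pawn has line of sight to the player.
; Each tick it traces on the Camera channel from the controlled pawn to slightly above the player's location, ignoring itself.
; When the trace hits the player, it writes the player actor and location to the blackboard.
; Otherwise it clears only the target key, leaving the last seen location intact.
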(event EventReceiveTickAI
  (params (OwnerController :type AI%20Controller%20Object%20Reference) (ControlledPawn :type Pawn%20Object%20Reference) (DeltaSeconds :type Float%20%28single-precision%29))
  (bind _returnvalue (Game|Player|GetPlayerPawn 0))
  (bind _targetplayerkey (Variables|Default|GetTargetPlayerKey))
  (bind _returnvalue_2 (Transformation|GetActorLocation _returnvalue))
  (bind _outhit (Collision|LineTraceByChannel (Transformation|GetActorLocation ControlledPawn) (+ _returnvalue_2 "0, 0,20.000000") "TraceTypeQuery2" false (Utilities|Array|MakeArray ControlledPawn) "None"))
  (if (== _returnvalue (.hitactor _outhit))
    (Class|BTFunctionLibrary|SetBlackboardValueasObject _targetplayerkey _returnvalue)
    (AI|BehaviorTree|SetBlackboardValueasVector (Variables|Default|GetPlayerLocationKey) _returnvalue_2)
    (else
      (Class|BTFunctionLibrary|ClearBlackboardValue _targetplayerkey))))