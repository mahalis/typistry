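; Behavior tree task that makes an enemy leap toward the player.
; On execute it casts the pawn to EnemyBase, calls Jump, then overwrites movement velocity with a fixed-speed, horizontal-only direction toward player 0.
; It reports success immediately without waiting for landing; a failed cast never calls FinishExecute.
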(event EventReceiveExecuteAI
  (params (OwnerController :type AI%20Controller%20Object%20Reference) (ControlledPawn :type Pawn%20Object%20Reference))
  (bind _returnvalue (Game|Player|GetPlayerPawn 0))
  (bind _returnvalue_2 (Transformation|GetActorLocation ControlledPawn))
  (bind _returnvalue_3 (Transformation|GetActorLocation _returnvalue))
  (bind _returnvalue_4 (- _returnvalue_3 _returnvalue_2))
  (bind _asenemy_base (Utilities|Casting|CastToEnemyBase ControlledPawn))
  (Character|Jump _asenemy_base)
  (Variables|/Script/Engine.MovementComponent|SetVelocity (Variables|/Script/Engine.Character|GetCharacterMovement _asenemy_base) (* (Math|Vector|Normalize (Math|Vector|MakeVector (.x _returnvalue_4) (.y _returnvalue_4) 0.0)) 3e+02))
  (AI|BehaviorTree|FinishExecute true))