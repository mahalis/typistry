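; Game mode for a typing-based enemy game, managing word lists, enemy spawning and the start, play and game-over flow.
; On BeginPlay it loads comma-separated word files bucketed by length, caches spawn points and creates both menu screens.
; StartGame spawns an initial wave, then random enemies on a looping timer until EndGame.
; Typing mode slows global time, and returning to the start screen destroys remaining enemies.
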(event EventBeginPlay
  (CallFunction|LoadWords)
  (CallFunction|FindSpawns)
  (bind _returnvalue (UserInterface|CreateWidget "/Game/Blueprints/UI/StartScreen.StartScreen_C"))
  (bind _output_get (Variables|Default|SetStartScreen _returnvalue))
  (UserInterface|Viewport|AddtoViewport _output_get 1)
  (bind _returnvalue_2 (UserInterface|CreateWidget "/Game/Blueprints/UI/GameOverScreen.GameOverScreen_C"))
  (bind _output_get_2 (Variables|Default|SetEndScreen _returnvalue_2))
  (UserInterface|Viewport|AddtoViewport _output_get_2 1)
  (Widget|SetVisibility _output_get_2 "Hidden")
  (Input|SetInputModeUIOnly (Game|GetPlayerController 0) _output_get "DoNotLock"))

(event EventTick
  (params (DeltaSeconds :type Float%20%28single-precision%29)))

(fn ConstructionScript)

(fn GetWordList
  (params (Length :type Integer))
  (switch int Length
    (:3
      (return (Variables|Default|GetWords3)))
    (:4
      (return (Variables|Default|GetWords4)))
    (:5
      (return (Variables|Default|GetWords5)))
    (:6
      (return (Variables|Default|GetWords6)))
    (:7
      (return (Variables|Default|GetWords7)))
    (:8
      (return (Variables|Default|GetWords8)))
    (:9
      (return (Variables|Default|GetWords9)))
    (:10
      (return (Variables|Default|GetWords10)))
    (:11
      (return (Variables|Default|GetWords11)))
    (:12
      (return (Variables|Default|GetWords12)))))

(fn LoadWords
  (for _index (range 3 12)
    (bind _returnvalue (Class|TextLoaderComponent|ReadFile (Variables|Default|GetTextLoader) (Utilities|String|BuildString(Integer) "" "words" _index ".txt")))
    (switch int _index
      (:3
        (Variables|Default|SetWords3 (Utilities|String|ParseIntoArray _returnvalue ",")))
      (:4
        (Variables|Default|SetWords4 (Utilities|String|ParseIntoArray _returnvalue ",")))
      (:5
        (Variables|Default|SetWords5 (Utilities|String|ParseIntoArray _returnvalue ",")))
      (:6
        (Variables|Default|SetWords6 (Utilities|String|ParseIntoArray _returnvalue ",")))
      (:7
        (Variables|Default|SetWords7 (Utilities|String|ParseIntoArray _returnvalue ",")))
      (:8
        (Variables|Default|SetWords8 (Utilities|String|ParseIntoArray _returnvalue ",")))
      (:9
        (Variables|Default|SetWords9 (Utilities|String|ParseIntoArray _returnvalue ",")))
      (:10
        (Variables|Default|SetWords10 (Utilities|String|ParseIntoArray _returnvalue ",")))
      (:11
        (Variables|Default|SetWords11 (Utilities|String|ParseIntoArray _returnvalue ",")))
      (:12
        (Variables|Default|SetWords12 (Utilities|String|ParseIntoArray _returnvalue ","))))))

(fn RandomWordfromWordList
  (params (Length :type Integer))
  (bind _list (CallFunction|GetWordList Length))
  (return (Utilities|Array|Get(acopy) _list (Math|Random|RandomInteger (- (Utilities|Array|Length _list) 1)))))

(fn FindSpawns
  (bind _outactors (Actor|GetAllActorsOfClass "/Game/Blueprints/Enemy/EnemySpawnPoint.EnemySpawnPoint_C"))
  (Variables|Default|SetEnemySpawns _outactors))

(fn SpawnEnemy
  (bind _enemyclasses (LocalVariables|GetEnemyClasses))
  (bind _enemyspawns (Variables|Default|GetEnemySpawns))
  (Game|SpawnActorfromClass (Utilities|Array|Get(acopy) _enemyclasses (Math|Random|RandomIntegerinRange 0 (- (Utilities|Array|Length _enemyclasses) 1))) (Math|Transform|MakeTransform (Transformation|GetWorldLocation (Variables|/Game/Blueprints/Enemy/EnemySpawnPoint.EnemySpawnPoint_C|GetDefaultSceneRoot (Utilities|Array|Get(acopy) _enemyspawns (Math|Random|RandomInteger (- (Utilities|Array|Length _enemyspawns) 1))))) "0, 0, 0" "1,1,1") "Undefined" 0 0))

(fn SetinTypingMode
  (params (Typing :type Boolean))
  (bind _output_get (Variables|Default|SetInTypingMode Typing))
  (Utilities|Time|SetGlobalTimeDilation (select _output_get 0.25 1.0)))

(fn EndGame
  (bind _endscreen (Variables|Default|GetEndScreen))
  (Variables|Default|SetIsPlaying false)
  (Variables|Default|SetIsGameOver true)
  (Utilities|Time|ClearTimerbyFunctionName 0 "SpawnEnemy")
  (Widget|SetVisibility _endscreen "Visible")
  (Input|SetInputModeUIOnly (Game|GetPlayerController 0) _endscreen "DoNotLock")
  (Variables|/Script/Engine.MovementComponent|SetVelocity (Pawn|GetMovementComponent (Game|Player|GetPlayerPawn 0)) "0, 0, 0"))

(fn StartGame
  (Variables|Default|SetIsPlaying true)
  (Variables|Default|SetIsGameOver false)
  (for _index (range 0 4)
    (CallFunction|SpawnEnemy))
  (Utilities|Time|SetTimerbyFunctionName 0 "SpawnEnemy" 3.0 true)
  (Input|SetInputModeGameOnly (Game|GetPlayerController 0))
  (Widget|SetVisibility (Variables|Default|GetStartScreen) "Hidden")
  (bind _asword_character (Utilities|Casting|CastToWordCharacter (Game|Player|GetPlayerPawn 0)))
  (Widget|SetVisibility (Variables|/Game/Blueprints/WordCharacter.WordCharacter_C|GetHUDWidget _asword_character) "Visible")
  (Variables|/Game/Blueprints/WordCharacter.WordCharacter_C|SetHealth _asword_character 100)
  (Audio|PlaySound2D "/Game/Sound/BackgroundMusic.BackgroundMusic"))

(fn ReturntoStartScreen
  (Widget|SetVisibility (Variables|Default|GetStartScreen) "Visible")
  (Widget|SetVisibility (Variables|Default|GetEndScreen) "Hidden")
  (bind _outactors (Actor|GetAllActorsOfClass "/Game/Blueprints/Enemy/EnemyBase.EnemyBase_C"))
  (for _array_element _outactors
    (Actor|DestroyActor _array_element)))